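; Pickup actor that hides itself and plays a 2D sound with randomized pitch when another actor overlaps it.
; The overlap event does not filter the other actor, and the actor is hidden rather than destroyed.
; A Gate passes the sound, then closes after a short delay to block later replays.
; Delay-based loops that poll for player overlap are left unconnected and never run.
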(event EventBeginPlay)

(event Collision|EventActorBeginOverlap
  (params (OtherActor :type Actor%20Object%20Reference))
  (Utilities|FlowControl|Sequence
    (:then_0
      (Rendering|SetActorHiddenInGame true)
      (Utilities|FlowControl|Gate false :!label _label
        (:Exit
          (Audio|PlaySound2D "/Game/6164105467527168.6164105467527168" 1.0 (Math|Random|RandomFloatinRange 0.8 1.4) 0.0 0 0))))
    (:then_1
      (Utilities|FlowControl|Delay 0.2)
      (goto _label Close))))

(event EventTick
  (params (DeltaSeconds :type Float%20%28single-precision%29)))

(fn ConstructionScript)